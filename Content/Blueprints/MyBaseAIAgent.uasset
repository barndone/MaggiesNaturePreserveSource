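; Base AI agent Blueprint that runs the BT_Seacoon behavior tree and mirrors its IsAwake state into the blackboard.
; On BeginPlay it casts its controller to BaseAIController, binds to ShouldUpdateBlackboard, starts the tree and writes the initial IsAwake value.
; Each dispatcher call rewrites that key, using a BBData helper that returns the blackboard and key name.
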(event `self.ReceiveBeginPlay`
  (bind (_returnvalue _returnvalue2) (`self.BB_Data` "IsAwake"))
  (bind _asbase_aicontroller (cast `BaseAIController` (`AIBlueprintHelperLibrary.GetAIController` self)))
  (add `BaseAIController.ShouldUpdateBlackboard` _asbase_aicontroller (delegate `OnTagUpdate_Event_0`))
  (`AIController.RunBehaviorTree` _asbase_aicontroller "/Game/MBP/AI/BT_Seacoon.BT_Seacoon")
  (`BlackboardComponent.SetValueAsBool` _returnvalue _returnvalue2 (`self.IsAwake`)))

(event `OnTagUpdate_Event_0`
  (bind (_returnvalue _returnvalue2) (`self.BB_Data` "IsAwake"))
  (`BlackboardComponent.SetValueAsBool` _returnvalue _returnvalue2 (`self.IsAwake`)))

(fn `BB_Data`
  (params (KeyName :type Name))
  (returns (ReturnValue :type "BlackboardComponent Object Reference") (ReturnValue2 :type Name))
  (return (`AIBlueprintHelperLibrary.GetBlackboard` (`AIBlueprintHelperLibrary.GetAIController` self)) (`KismetSystemLibrary.MakeLiteralName` KeyName)))

(fn `UserConstructionScript`)