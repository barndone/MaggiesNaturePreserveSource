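; BP_SokobonGrid is a Sokobon puzzle grid Blueprint that adds audio feedback when the puzzle is completed.
; On BeginPlay it binds to its puzzle-complete event and the Audio component's finished event.
; Completion plays JingleLoop, and any audio finish switches to JingleEnd and plays it, including when JingleEnd itself finishes.
; The graph holds no grid or movement logic, and the construction script is empty.
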(event `self.ReceiveBeginPlay`
  (add `self.OnPuzzleComplete` (delegate `OnPuzzleComplete_Event_0`))
  (add `AudioComponent.OnAudioFinished` (`self.Audio`) (delegate `OnAudioFinished_Event_0`)))

(event `OnPuzzleComplete_Event_0` :!signature `self.OnPuzzleComplete`
  (params (_completedPuzzle :type "ACSokobonGrid Object Reference"))
  (`AudioComponent.SetSound` (`self.Audio`) (`self.JingleLoop`))
  (`AudioComponent.Play` (`self.Audio`) 0.0))

(event `OnAudioFinished_Event_0`
  (`AudioComponent.SetSound` (`self.Audio`) (`self.JingleEnd`))
  (`AudioComponent.Play` (`self.Audio`) 0.0))

(fn `UserConstructionScript`)