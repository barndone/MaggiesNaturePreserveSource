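; Pushable Sokoban puzzle piece that adds sound, particle and UI feedback on top of a C++ backend.
; Move, fall and hole-fill delegates drive pitch-randomized sounds, with particles active from move start until the piece move event.
; A trigger shows an input prompt widget while the ThirdPersonCharacter overlaps it.
; A separate tutorial indicator, toggled by show/hide functions, bobs on a sine wave in Tick.
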(event `self.ReceiveBeginPlay`
  (bind _tutorialindicatorwidget (`self.TutorialIndicatorWidget`))
  ;[1 1 1] Example sound implementation with the C++ backend
  (add `self.OnMoveStart` (delegate `CustomEvent_0`))
  (`SceneComponent.SetHiddenInGame` _tutorialindicatorwidget true false)
  (`ActorComponent.SetComponentTickEnabled` _tutorialindicatorwidget false)
  (bind _asacinput_prompt (cast `ACInputPrompt` (`WidgetComponent.GetUserWidgetObject` (`self.UIPopUpWidget`))))
  (`ACInputPrompt.SetParent` _asacinput_prompt self)
  (`ACInputPrompt.BindCharacterEvents` _asacinput_prompt)
  (add `self.OnPieceMove` (delegate `PS STOP`))
  (`ActorComponent.SetActive` (`self.ParticleSystem`) false false)
  (add `self.OnFallStart` (delegate `fall start`))
  (add `self.OnHoleFill` (delegate `on fall complete`)))

(event `on fall complete` :!signature `self.OnHoleFill`
  (params (_curTile :type "ACSokobonTile Object Reference"))
  (`GameplayStatics.PlaySoundAtLocation` (`self.FallComplete`) (`self.K2_GetActorLocation`) (struct) 1.0 (`KismetMathLibrary.RandomFloatInRange` 0.5 1.5) 0.0 null null null))

(event `CustomEvent_0`
  ;[1 1 1] Example sound implementation with the C++ backend
  (`GameplayStatics.PlaySoundAtLocation` (`self.PushPullSound`) (`self.K2_GetActorLocation`) (struct) 1.0 (`KismetMathLibrary.RandomFloatInRange` 0.5 1.0) 0.0 null null null)
  (`ActorComponent.SetActive` (`self.ParticleSystem`) true false))

(event `fall start` :!signature `self.OnFallStart`
  (params (_hole :type "ACSokobonHole Object Reference"))
  (`GameplayStatics.PlaySoundAtLocation` (`self.FallSound`) (`self.K2_GetActorLocation`) (struct) 1.0 (`KismetMathLibrary.RandomFloatInRange` 0.5 1.5) 0.0 null null null))

(event `PS STOP`
  (`ActorComponent.SetActive` (`self.ParticleSystem`) false false))

(event `self.ReceiveTick`
  (params (DeltaSeconds :type "Float (single-precision)"))
  (`SceneComponent.K2_AddLocalOffset` (`self.TutorialIndicatorWidget`) (`KismetMathLibrary.MakeVector` 0.0 0.0 (* DeltaSeconds (`self.TutorialPromptAmp`) (`KismetMathLibrary.Sin` (* (`GameplayStatics.GetRealTimeSeconds`) (`self.wavelength`))))) false false))

(event `self.Trigger.OnComponentBeginOverlap`
  (params (OverlappedComponent :type "PrimitiveComponent Object Reference") (OtherActor :type "Actor Object Reference") (OtherComp :type "PrimitiveComponent Object Reference") (OtherBodyIndex :type Integer) (bFromSweep :type Boolean) (SweepResult :type "HitResult Structure (by ref)"))
  ;[1 1 1] UIPopUpCode
  (cast `/Game/MBP/Core/ThirdPersonCharacter` OtherActor)
  (`SceneComponent.SetHiddenInGame` (`self.UIPopUpWidget`) false false))

(event `self.Trigger.OnComponentEndOverlap`
  (params (OverlappedComponent :type "PrimitiveComponent Object Reference") (OtherActor :type "Actor Object Reference") (OtherComp :type "PrimitiveComponent Object Reference") (OtherBodyIndex :type Integer))
  ;[1 1 1] UIPopUpCode
  (cast `/Game/MBP/Core/ThirdPersonCharacter` OtherActor)
  (`SceneComponent.SetHiddenInGame` (`self.UIPopUpWidget`) true false))

(fn `HideTutorialPrompt`
  (bind _tutorialindicatorwidget (`self.TutorialIndicatorWidget`))
  (`SceneComponent.SetHiddenInGame` _tutorialindicatorwidget true false)
  (`ActorComponent.SetComponentTickEnabled` _tutorialindicatorwidget false))

(fn `ShowTutorialPrompt`
  (bind _tutorialindicatorwidget (`self.TutorialIndicatorWidget`))
  (`SceneComponent.SetHiddenInGame` _tutorialindicatorwidget false false)
  (`ActorComponent.SetComponentTickEnabled` _tutorialindicatorwidget true))

(fn `UserConstructionScript`)