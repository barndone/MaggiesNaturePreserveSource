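; BP_Rolling_Block is the presentation layer for a movable block that can be pushed or pulled, ride conveyors and fall into holes.
; It binds inherited movement events to pitch-randomized sounds and toggles a particle effect, swapping its template when a conveyor starts.
; A trigger shows an input-prompt widget when the ThirdPersonCharacter enters and hides it when any overlap ends, since that cast is disconnected.
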(event `self.ReceiveBeginPlay`
  (bind _asacinput_prompt (cast `ACInputPrompt` (`WidgetComponent.GetUserWidgetObject` (`self.UIPopUpWidget`))))
  (`ACInputPrompt.SetParent` _asacinput_prompt self)
  (`ACInputPrompt.BindCharacterEvents` _asacinput_prompt)
  (add `self.OnMoveStart` (delegate `CustomEvent_0`))
  (add `self.OnPieceMove` (delegate `PS STOP`))
  (`ActorComponent.SetActive` (`self.ParticleSystem`) false false)
  (add `self.OnConveyorStart` (delegate `conveyorstart`))
  (add `self.OnHoleFill` (delegate `holefallevent`))
  (add `self.OnFallStart` (delegate `fall start`)))

(event `fall start` :!signature `self.OnFallStart`
  (params (_hole :type "ACSokobonHole Object Reference"))
  (`GameplayStatics.PlaySoundAtLocation` (`self.fallStart`) (`self.K2_GetActorLocation`) (struct) 1.0 (`KismetMathLibrary.RandomFloatInRange` 0.5 1.5) 0.0 null null null))

(event `CustomEvent_0`
  (`GameplayStatics.PlaySoundAtLocation` (`self.PushPullSound`) (`self.K2_GetActorLocation`) (struct) 1.0 (`KismetMathLibrary.RandomFloatInRange` 0.5 1.0) 0.0 null null null)
  (`ActorComponent.SetActive` (`self.ParticleSystem`) true false))

(event `holefallevent` :!signature `self.OnHoleFill`
  (params (_curTile :type "ACSokobonTile Object Reference"))
  (`GameplayStatics.PlaySoundAtLocation` (`self.FallSound`) (`self.K2_GetActorLocation`) (struct) 1.0 (`KismetMathLibrary.RandomFloatInRange` 0.5 1.5) 0.0 null null null))

(event `PS STOP`
  (`ActorComponent.SetActive` (`self.ParticleSystem`) false false))

(event `conveyorstart`
  (`ParticleSystemComponent.SetTemplate` (`self.ParticleSystem`) (`self.PSTemplateSea`)))

(event `self.Trigger.OnComponentBeginOverlap`
  (params (OverlappedComponent :type "PrimitiveComponent Object Reference") (OtherActor :type "Actor Object Reference") (OtherComp :type "PrimitiveComponent Object Reference") (OtherBodyIndex :type Integer) (bFromSweep :type Boolean) (SweepResult :type "HitResult Structure (by ref)"))
  (cast `/Game/MBP/Core/ThirdPersonCharacter` OtherActor)
  (`SceneComponent.SetHiddenInGame` (`self.UIPopUpWidget`) false false))

(event `self.Trigger.OnComponentEndOverlap`
  (params (OverlappedComponent :type "PrimitiveComponent Object Reference") (OtherActor :type "Actor Object Reference") (OtherComp :type "PrimitiveComponent Object Reference") (OtherBodyIndex :type Integer))
  (`SceneComponent.SetHiddenInGame` (`self.UIPopUpWidget`) true false))

(fn `UserConstructionScript`)