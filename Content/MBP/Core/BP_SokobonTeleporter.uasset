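; Sokoban teleporter Blueprint that shows whether it is blocked by scaling its portal plane.
; Blocked and unblocked events start a Tick-driven lerp toward the blocked or final scale, stopping within a tolerance.
; Shortly after BeginPlay, an already blocked teleporter shrinks to its blocked scale.
; A separate trigger volume slows the third-person character's camera lag on entry and raises its speed again on exit.
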(event `self.ReceiveBeginPlay`
  (add `self.OnTeleportBlocked` (delegate `OnTeleportBlock`))
  (add `self.OnTeleportUnblocked` (delegate `UnTeleportUnBlock`))
  (`KismetSystemLibrary.Delay` 0.2)
  (if (`self.Blocked`)
    (set `self.bStartTransition` true)
    (set `self.bIsGrowing` false)))

(event `OnTeleportBlock`
  (set `self.bStartTransition` true)
  (set `self.bIsGrowing` false))

(event `UnTeleportUnBlock`
  (set `self.bStartTransition` true)
  (set `self.bIsGrowing` true))

(event `self.ReceiveTick`
  (params (DeltaSeconds :type "Float (single-precision)"))
  (if (`self.bStartTransition`)
    (set `self.LerpTimer` (+ DeltaSeconds (`self.LerpTimer`)))
    (if (`self.bIsGrowing`)
      ;[1 1 1] Lerp to the desired teleport viz scale
      (`SceneComponent.SetWorldScale3D` (`self.Portal_plane`) (`KismetMathLibrary.VLerp` (`SceneComponent.K2_GetComponentScale` (`self.Portal_plane`)) (`self.FinalPortalScale`) (/ (`self.LerpTimer`) (`self.LerpTimeDur`))))
      (if (`KismetMathLibrary.Vector_IsNearlyZero` (- (`self.FinalPortalScale`) (`SceneComponent.K2_GetComponentScale` (`self.Portal_plane`))) 0.1)
        (set `self.bStartTransition` false)
        (set `self.LerpTimer` 0.0))
      (else
        (`SceneComponent.SetWorldScale3D` (`self.Portal_plane`) (`KismetMathLibrary.VLerp` (`SceneComponent.K2_GetComponentScale` (`self.Portal_plane`)) (`self.BlockedPortalScale`) (/ (`self.LerpTimer`) (`self.LerpTimeDur`))))
        (if (`KismetMathLibrary.Vector_IsNearlyZero` (- (`self.BlockedPortalScale`) (`SceneComponent.K2_GetComponentScale` (`self.Portal_plane`))) 0.1)
          (set `self.bStartTransition` false)
          (set `self.LerpTimer` 0.0))))))

(event `self.CamLagTrigger.OnComponentBeginOverlap`
  (params (OverlappedComponent :type "PrimitiveComponent Object Reference") (OtherActor :type "Actor Object Reference") (OtherComp :type "PrimitiveComponent Object Reference") (OtherBodyIndex :type Integer) (bFromSweep :type Boolean) (SweepResult :type "HitResult Structure (by ref)"))
  (bind _asthird_person_character (cast `/Game/MBP/Core/ThirdPersonCharacter` OtherActor))
  (bind _cameraboom (`AControlCharacter.CameraBoom` _asthird_person_character))
  (set `SpringArmComponent.bEnableCameraLag` true _cameraboom)
  (set `SpringArmComponent.CameraLagSpeed` 0.8 _cameraboom))

(event `self.CamLagTrigger.OnComponentEndOverlap`
  (params (OverlappedComponent :type "PrimitiveComponent Object Reference") (OtherActor :type "Actor Object Reference") (OtherComp :type "PrimitiveComponent Object Reference") (OtherBodyIndex :type Integer))
  (bind _asthird_person_character (cast `/Game/MBP/Core/ThirdPersonCharacter` OtherActor))
  (set `SpringArmComponent.CameraLagSpeed` 10.0 (`AControlCharacter.CameraBoom` _asthird_person_character)))

(fn `UserConstructionScript`)