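; Sokoban puzzle hole actor that shows a dust effect and carries a tutorial prompt widget.
; On BeginPlay it hides both components and binds a show-dust callback, which after a short delay spawns the hidden particle component's template just above the hole.
; Show and hide functions toggle the widget's visibility and component tick, while the actor's Tick continuously bobs it vertically with a time-based sine offset.
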(event `self.ReceiveBeginPlay`
  (bind _tutorialindicatorwidget (`self.TutorialIndicatorWidget`))
  (`SceneComponent.SetHiddenInGame` _tutorialindicatorwidget true false)
  (`ActorComponent.SetComponentTickEnabled` _tutorialindicatorwidget false)
  (`SceneComponent.SetHiddenInGame` (`self.ParticleSystem`) true false)
  (add `self.ShowDust` (delegate `spawn_dust`)))

(event `spawn_dust`
  ;[1 1 1] Comment
  (`KismetSystemLibrary.Delay` 0.45)
  (`GameplayStatics.SpawnEmitterAtLocation` (`ParticleSystemComponent.Template` (`self.ParticleSystem`)) (+ (`self.K2_GetActorLocation`) (0.0 0.0 30.0))))

(event `self.ReceiveTick`
  (params (DeltaSeconds :type "Float (single-precision)"))
  (`SceneComponent.K2_AddLocalOffset` (`self.TutorialIndicatorWidget`) (`KismetMathLibrary.MakeVector` 0.0 0.0 (* DeltaSeconds (`self.Tutorial Prompt Amp`) (`KismetMathLibrary.Sin` (* (`GameplayStatics.GetRealTimeSeconds`) (`self.wavelength`))))) false false))

(fn `HideTutorialPrompt`
  (bind _tutorialindicatorwidget (`self.TutorialIndicatorWidget`))
  (`SceneComponent.SetHiddenInGame` _tutorialindicatorwidget true false)
  (`ActorComponent.SetComponentTickEnabled` _tutorialindicatorwidget false))

(fn `ShowTutorialPrompt`
  (bind _tutorialindicatorwidget (`self.TutorialIndicatorWidget`))
  (`SceneComponent.SetHiddenInGame` _tutorialindicatorwidget false false)
  (`ActorComponent.SetComponentTickEnabled` _tutorialindicatorwidget true))

(fn `UserConstructionScript`)