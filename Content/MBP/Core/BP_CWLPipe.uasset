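; BP_CWLPipe is an interactable pipe actor that shows an input prompt near the player and plays sounds when it starts moving.
; On BeginPlay it passes itself to its ACInputPrompt widget, has it bind character events, and binds its move-start event.
; Trigger overlaps with a ThirdPersonCharacter show or hide the popup widget.
; Each move start plays a random sound at the mesh's location.
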(event `OnMove`
  (`GameplayStatics.PlaySoundAtLocation` (`KismetArrayLibrary.Array_Random` (`self.Sounds`)) (`SceneComponent.K2_GetComponentLocation` (`self.Mesh`)) (struct) 1.0 1.0 0.0 null null null))

(event `self.ReceiveBeginPlay`
  (bind _asacinput_prompt (cast `ACInputPrompt` (`WidgetComponent.GetUserWidgetObject` (`self.UIPopUpWidget`))))
  (`ACInputPrompt.SetParent` _asacinput_prompt self)
  (`ACInputPrompt.BindCharacterEvents` _asacinput_prompt)
  (add `self.OnMoveStart` (delegate `OnMove`)))

(event `self.Trigger.OnComponentBeginOverlap`
  (params (OverlappedComponent :type "PrimitiveComponent Object Reference") (OtherActor :type "Actor Object Reference") (OtherComp :type "PrimitiveComponent Object Reference") (OtherBodyIndex :type Integer) (bFromSweep :type Boolean) (SweepResult :type "HitResult Structure (by ref)"))
  (cast `/Game/MBP/Core/ThirdPersonCharacter` OtherActor)
  (`SceneComponent.SetHiddenInGame` (`self.UIPopUpWidget`) false false))

(event `self.Trigger.OnComponentEndOverlap`
  (params (OverlappedComponent :type "PrimitiveComponent Object Reference") (OtherActor :type "Actor Object Reference") (OtherComp :type "PrimitiveComponent Object Reference") (OtherBodyIndex :type Integer))
  (cast `/Game/MBP/Core/ThirdPersonCharacter` OtherActor)
  (`SceneComponent.SetHiddenInGame` (`self.UIPopUpWidget`) true false))

(fn `UserConstructionScript`)