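; BP_SokobonGoal is a goal actor, named for a Sokoban-style puzzle, with a toggleable tutorial indicator and recurring ambient sound.
; The indicator widget starts hidden with tick disabled, and the Show and Hide functions switch both.
; Tick bobs the widget vertically with a real-time sine offset.
; Tick also runs a timer that replays the sound at random intervals, at world origin rather than the actor's location.
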(event `self.ReceiveBeginPlay`
  (bind _tutorialindicatorwidget (`self.TutorialIndicatorWidget`))
  (`SceneComponent.SetHiddenInGame` _tutorialindicatorwidget true false)
  (`ActorComponent.SetComponentTickEnabled` _tutorialindicatorwidget false))

(event `self.ReceiveTick`
  (params (DeltaSeconds :type "Float (single-precision)"))
  (`self.RandomlyPlaySound` DeltaSeconds)
  (`SceneComponent.K2_AddLocalOffset` (`self.TutorialIndicatorWidget`) (`KismetMathLibrary.MakeVector` 0.0 0.0 (* DeltaSeconds (`self.TutorialPromptAmp`) (`KismetMathLibrary.Sin` (* (`GameplayStatics.GetRealTimeSeconds`) (`self.wavelength`))))) false false))

(fn `HideTutorialPrompt`
  (bind _tutorialindicatorwidget (`self.TutorialIndicatorWidget`))
  (`SceneComponent.SetHiddenInGame` _tutorialindicatorwidget true false)
  (`ActorComponent.SetComponentTickEnabled` _tutorialindicatorwidget false))

(fn `RandomlyPlaySound`
  (params (DeltaTime :type "Float (double-precision)"))
  (bind _output_get (set `self.RandomSoundTimer` (+ DeltaTime (`self.RandomSoundTimer`))))
  (if (>= _output_get (`self.RandomSoundDelay`))
    (`GameplayStatics.PlaySoundAtLocation` (`self.Sound`) (0.0 0.0 0.0) (struct) 1.0 1.0 0.0 null null null)
    (set `self.RandomSoundDelay` (`KismetMathLibrary.RandomFloatInRange` (`self.MinSoundDelay`) (`self.MaxSoundDelay`)))
    (set `self.RandomSoundTimer` 0.0)
    (return)
    (else
      (return))))

(fn `ShowTutorialPrompt`
  (bind _tutorialindicatorwidget (`self.TutorialIndicatorWidget`))
  (`SceneComponent.SetHiddenInGame` _tutorialindicatorwidget false false)
  (`ActorComponent.SetComponentTickEnabled` _tutorialindicatorwidget true))

(fn `UserConstructionScript`)